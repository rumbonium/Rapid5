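; Rat King boss actor that alternates between facing two player directions and loses health to crow bow projectile hits.
; Tick yaws it at a set speed to the target rotation, then a random-length timer triggers the next turn.
; Child enemy spawners pause during turns, retarget to the faced player and resume on arrival.
; Hits update a health bar widget; zero health calls BossDestroyed and destroys the actor.
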(event EventBeginPlay
  (Variables|Gameplay|SetRotationTarget (Math|Rotator|SelectRotator (Variables|Gameplay|GetP0Rotation) (Variables|Gameplay|GetP1Rotation) (== (Math|Random|RandomIntegerinRange 0 1) 0)))
  (CallFunction|TimetoRotateTimerExpired)
  (bind _returnvalue (UserInterface|CreateWidget "/Game/Widgets/WBP_BossHealthBar.WBP_BossHealthBar_C"))
  (bind _output_get (Variables|Gameplay|SetWBP_HealthBar _returnvalue))
  (UserInterface|Viewport|AddtoViewport _output_get 0)
  (Variables|Gameplay|SetBossHealth (Variables|Gameplay|GetBossMaxHealth))
  (Progress|SetPercent (Variables|/Game/Widgets/WBP_BossHealthBar.WBP_BossHealthBar_C|GetHealthBar (Variables|Gameplay|GetWBP_HealthBar)) 1.0))

(event Collision|EventHit
  (params (MyComp :type Primitive%20Component%20Object%20Reference) (Other :type Actor%20Object%20Reference) (OtherComp :type Primitive%20Component%20Object%20Reference) (bSelfMoved :type Boolean) (HitLocation :type Vector :default "0, 0, 0") (HitNormal :type Vector :default "0, 0, 0") (NormalImpulse :type Vector :default "0, 0, 0") (Hit :type Hit%20Result%20Structure%20%28by%20ref%29))
  (Utilities|Casting|CastToCrowsBowProjectile Other)
  (Variables|Gameplay|SetBossHealth (- (Variables|Gameplay|GetBossHealth) 1.0))
  (Progress|SetPercent (Variables|/Game/Widgets/WBP_BossHealthBar.WBP_BossHealthBar_C|GetHealthBar (Variables|Gameplay|GetWBP_HealthBar)) (/ (Variables|Gameplay|GetBossHealth) (Variables|Gameplay|GetBossMaxHealth)))
  (if (== 0.0 (Variables|Gameplay|GetBossHealth))
    (Default|CallBossDestroyed)
    (Widget|RemovefromParent (Variables|Gameplay|GetWBP_HealthBar))
    (Actor|DestroyActor)))

(event EventTick
  (params (DeltaSeconds :type Float%20%28single-precision%29))
  (bind _returnvalue (Transformation|GetActorRotation))
  (bind (_roll _pitch _yaw) (Math|Rotator|BreakRotator _returnvalue))
  (if (Variables|Gameplay|GetIsRotating?)
    (Transformation|SetActorRotation (Math|Interpolation|RInterpTo _returnvalue (Math|Rotator|MakeRotator _roll _pitch (+ _yaw (* DeltaSeconds (Variables|Gameplay|GetRotationSpeed)))) DeltaSeconds 0.0))
    (if (Math|Rotator|Equal(Rotator) (Transformation|GetActorRotation) (Variables|Gameplay|GetRotationTarget) (Variables|Gameplay|GetrotationTolerance))
      (Variables|Gameplay|SetIsRotating? false)
      (Utilities|Time|SetTimerbyFunctionName 0 "TimeToRotateTimerExpired" (Math|Random|RandomFloatinRange (Variables|Gameplay|GetMinTimeBeforeRotate) (Variables|Gameplay|GetMaxTimeBeforeRotate)))
      (for _array_element (Actor|GetAllChildActors false)
        (if (== (Utilities|GetClass _array_element) "/Game/Blueprints/BP_EnemySpawner.BP_EnemySpawner_C")
          (bind _asbp_enemy_spawner (Utilities|Casting|CastToBP_EnemySpawner _array_element))
          (Variables|/Game/Blueprints/BP_EnemySpawner.BP_EnemySpawner_C|SetSpawnAllowed? _asbp_enemy_spawner true))))))

(fn ConstructionScript)

(fn TimetoRotateTimerExpired
  (Variables|Gameplay|SetIsRotating? true)
  (Variables|Gameplay|SetRotationTarget (Math|Rotator|SelectRotator (Variables|Gameplay|GetP1Rotation) (Variables|Gameplay|GetP0Rotation) (Math|Rotator|Equal(Rotator) (Variables|Gameplay|GetRotationTarget) (Variables|Gameplay|GetP0Rotation) 0.0001)))
  (for _array_element (Actor|GetAllChildActors false)
    (if (== (Utilities|GetClass _array_element) "/Game/Blueprints/BP_EnemySpawner.BP_EnemySpawner_C")
      (bind _asbp_enemy_spawner (Utilities|Casting|CastToBP_EnemySpawner _array_element))
      (Variables|/Game/Blueprints/BP_EnemySpawner.BP_EnemySpawner_C|SetSpawnAllowed? _asbp_enemy_spawner false)
      (Variables|/Game/Blueprints/BP_EnemySpawner.BP_EnemySpawner_C|SetPlayerTarget _asbp_enemy_spawner (Math|Integer|SelectInt 0 1 (Math|Rotator|Equal(Rotator) (Variables|Gameplay|GetRotationTarget) (Variables|Gameplay|GetP0Rotation) 0.0001)))))
  (return))