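; BP_BasicEnemy is a simple chasing enemy that homes in on the player character selected by TargetPlayerNum.
; Each tick it moves straight toward that character at BaseSpeed, using a swept world offset rather than pathfinding.
; A hit from a CrowsBowProjectile reports the kill through BP_EnemyTracker's dispatcher, found by class lookup, then destroys the enemy.
; Hitting a TopDownCharacter is detected by a cast but triggers nothing.
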(event EventBeginPlay)

(event EventTick
  (params (DeltaSeconds :type Float%20%28single-precision%29))
  (Transformation|AddActorWorldOffset (* (* (Math|Vector|Normalize (- (Transformation|GetActorLocation (Game|GetPlayerCharacter (Variables|Default|GetTargetPlayerNum))) (Transformation|GetActorLocation))) (Variables|Default|GetBaseSpeed)) DeltaSeconds) true))

(event Collision|EventHit
  (params (MyComp :type Primitive%20Component%20Object%20Reference) (Other :type Actor%20Object%20Reference) (OtherComp :type Primitive%20Component%20Object%20Reference) (bSelfMoved :type Boolean) (HitLocation :type Vector :default "0, 0, 0") (HitNormal :type Vector :default "0, 0, 0") (NormalImpulse :type Vector :default "0, 0, 0") (Hit :type Hit%20Result%20Structure%20%28by%20ref%29))
  (Utilities|Casting|CastToCrowsBowProjectile Other
    (:then
      (bind _outactors (Actor|GetAllActorsOfClass "/Game/Blueprints/BP_EnemyTracker.BP_EnemyTracker_C"))
      (Default|CallEnemyKilledDispatcher _outactors (Variables|Default|GetTargetPlayerNum))
      (Actor|DestroyActor))
    (:CastFailed
      (Utilities|Casting|CastToTopDownCharacter Other))))

(fn ConstructionScript)