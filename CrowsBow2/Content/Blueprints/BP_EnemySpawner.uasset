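; Enemy spawner actor that periodically spawns enemies aimed at a specific player.
; A looping timer calls SpawnEnemies, which, while spawning is allowed, spawns a random class from the configured enemy list at the spawner's transform.
; Each spawned BP_BasicEnemy receives the target player number and a reduced scale, then the spawn is reported to BP_EnemyTracker for that player.
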(event Custom|SpawnEnemies
  (bind _enemytypestospawn (Variables|Gameplay|GetEnemyTypesToSpawn))
  (bind _playertarget (Variables|Gameplay|GetPlayerTarget))
  (if (Variables|Gameplay|GetSpawnAllowed?)
    (bind _returnvalue (Game|SpawnActorfromClass (Utilities|Array|Get(acopy) _enemytypestospawn (Math|Random|RandomIntegerinRange 0 (- (Utilities|Array|Length _enemytypestospawn) 1))) (Transformation|GetActorTransform self) "AlwaysSpawn" 0 0))
    (bind _asbp_basic_enemy (Utilities|Casting|CastToBP_BasicEnemy _returnvalue))
    (Variables|/Game/Blueprints/BP_BasicEnemy.BP_BasicEnemy_C|SetTargetPlayerNum _asbp_basic_enemy _playertarget)
    (Transformation|SetActorScale3D _asbp_basic_enemy "0.600000,0.600000,0.600000")
    (bind _outactors (Actor|GetAllActorsOfClass "/Game/Blueprints/BP_EnemyTracker.BP_EnemyTracker_C"))
    (Default|EnemySpawned _outactors _playertarget)))

(event EventBeginPlay
  (Utilities|Time|SetTimerbyFunctionName 0 "SpawnEnemies" (Variables|Gameplay|GetTimeBetweenSpawn) true))

(fn ConstructionScript)